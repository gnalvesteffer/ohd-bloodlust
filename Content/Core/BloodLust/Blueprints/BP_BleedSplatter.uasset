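; BP_BleedSplatter is a blood splatter decal actor that varies its look each time it is constructed.
; Its construction script creates a dynamic material on the SplatterDecal component and assigns a random texture from BloodTextures.
; It also passes the creation time and a drip amount, computed as the actor's up vector dotted with world up, so the material receives surface orientation.
; The event graph has no logic.
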(event `self.ReceiveBeginPlay`)

(fn `UserConstructionScript`
  (bind _bloodtextures (`self.BloodTextures`))
  (bind _returnvalue (`DecalComponent.CreateDynamicMaterialInstance` (`self.SplatterDecal`)))
  (`MaterialInstanceDynamic.SetTextureParameterValue` _returnvalue "Texture" (`|GetArrayItem` _bloodtextures (`KismetMathLibrary.RandomIntegerInRange` 0 (- (`KismetArrayLibrary.Array_Length` _bloodtextures) 1))))
  (`MaterialInstanceDynamic.SetScalarParameterValue` _returnvalue "CreateTime" (`GameplayStatics.GetTimeSeconds`))
  (`MaterialInstanceDynamic.SetScalarParameterValue` _returnvalue "DripAmount" (`KismetMathLibrary.Dot_VectorVector` (`self.GetActorUpVector`) (0.0 0.0 1.0))))