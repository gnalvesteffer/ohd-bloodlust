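; BloodLust ruleset that spawns blood splatters when registered actors take point damage.
; Hits at or above a damage threshold spawn a surface splatter along the shot direction, a ground splatter below and several mess splatters in random directions.
; A shared helper line-traces against WorldStatic objects, aligns each splatter to the impact normal and scales it by damage, trace distance and random variation.
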(event `HandlePointDamage`
  (params (DamagedActor :type "Actor Object Reference") (Damage :type "Float (double-precision)") (InstigatedBy :type "Controller Object Reference") (HitLocation :type "Vector Structure") (FHitComponent :type "PrimitiveComponent Object Reference") (BoneName :type Name) (ShotFromDirection :type "Vector Structure") (DamageType :type "DamageType Object Reference") (DamageCauser :type "Actor Object Reference"))
  (`self.OnCharacterHit` HitLocation ShotFromDirection Damage))

(event `self.RegisterActor`
  (params (RegisteredActor :type "Actor Object Reference"))
  (add `Actor.OnTakePointDamage` RegisteredActor (delegate `HandlePointDamage`)))

(fn `CalculateSplatterTransform`
  (params (HitPosition :type "Vector Structure") (HitDirection :type "Vector Structure") (Damage :type "Float (double-precision)") (MaxDistance :type "Float (double-precision)"))
  (returns (SplatterTransform :type "Transform Structure") (DidIntersect :type Boolean))
  (bind (_outhit _returnvalue) (`KismetSystemLibrary.LineTraceSingleForObjects` HitPosition (+ HitPosition (* HitDirection MaxDistance)) (`|MakeArray` "ObjectTypeQuery1" :!type "EObjectTypeQuery Enum")))
  (if _returnvalue
    (return (`KismetMathLibrary.MakeTransform` (`.ImpactPoint` (`GameplayStatics.BreakHitResult` _outhit)) (`KismetMathLibrary.Conv_VectorToRotator` (`.ImpactNormal` (`GameplayStatics.BreakHitResult` _outhit))) (* (+ (0.9 0.9 0.9) (* (0.2 0.2 0.2) (`KismetMathLibrary.RandomFloatInRange` 0.0 1.0))) (+ (`KismetMathLibrary.FMin` (* Damage 0.015) 1.25) (/ (`.Distance` (`GameplayStatics.BreakHitResult` _outhit)) 600.0)))) true)
    (else
      (return (struct) false))))

(fn `OnCharacterHit`
  (params (HitPosition :type "Vector Structure") (HitDirection :type "Vector Structure") (Damage :type "Float (double-precision)"))
  (bind (_splattertransform _didintersect) (`self.CalculateSplatterTransform` HitPosition (`KismetMathLibrary.RandomUnitVector`) Damage (`self.MaxMessDistanceCentimeters`)))
  (bind (_splattertransform_2 _didintersect_2) (`self.CalculateSplatterTransform` HitPosition (0.0 0.0 -1.0) Damage (`self.MaxSplatterDistanceCentimeters`)))
  (bind (_splattertransform_3 _didintersect_3) (`self.CalculateSplatterTransform` HitPosition HitDirection Damage (`self.MaxSplatterDistanceCentimeters`)))
  (if (>= Damage (`self.RequiredDamageForBloodSplatter`))
    (`|ExecutionSequence`
      (:`then_0`
        ;[1 1 1] Spawn Surface Splatter
        (if _didintersect_3
          (`|SpawnActorFromClass` "/XorberaxBloodLust/Core/BloodLust/Blueprints/BP_SurfaceSplatter.BP_SurfaceSplatter_C" _splattertransform_3 "AlwaysSpawn" "OverrideRootScale" null null)))
      (:`then_1`
        ;[1 1 1] Spawn Ground Splatter
        (if _didintersect_2
          (`|SpawnActorFromClass` "/XorberaxBloodLust/Core/BloodLust/Blueprints/BP_GroundSplatter.BP_GroundSplatter_C" _splattertransform_2 "AlwaysSpawn" "OverrideRootScale" null null)))
      (:`then_2`
        ;[1 1 1] Spawn Mess Splatters
        (for _ (range 1 (+ (`self.MessSplatterIterations`) 1))
          (if _didintersect
            (`|SpawnActorFromClass` "/XorberaxBloodLust/Core/BloodLust/Blueprints/BP_MessSplatter.BP_MessSplatter_C" _splattertransform "AlwaysSpawn" "OverrideRootScale" null null)))))))